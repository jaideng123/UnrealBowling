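; Bowling pin setter that spawns pins at BeginPlay and resets, clears or reports them when the game mode asks.
; It binds to BowlingGameMode_BP events, with a TODO to move that control into the game mode.
; Clearing raises standing pins, sweeps and lowers them on timed delays, then notifies the game mode.
; The sweep briefly enables a hidden Cube's collision and visibility while DueMove eases it out and back.
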(event `self.ReceiveBeginPlay`
  (`PrimitiveComponent.SetCollisionEnabled` (`self.Cube`) "NoCollision")
  (`SceneComponent.SetVisibility` (`self.Cube`) false true)
  (`self.SpawnPins`)
  (bind _asbowling_game_mode_bp (cast `/Game/BluePrints/BowlingGameMode_BP` (`GameplayStatics.GetGameMode`)))
  ;[1 1 1] TODO: Move Control of this to Game Mode
  (add `/Game/BluePrints/BowlingGameMode_BP.StartNextTurn` _asbowling_game_mode_bp (delegate `OnStartNextTurn`))
  (add `/Game/BluePrints/BowlingGameMode_BP.ClearPins` _asbowling_game_mode_bp (delegate `OnClearPins`))
  (add `/Game/BluePrints/BowlingGameMode_BP.ReportPins` _asbowling_game_mode_bp (delegate `OnReportPins`))
  (add `/Game/BluePrints/BowlingGameMode_BP.QuickResetPins` _asbowling_game_mode_bp (delegate `QuickResetPins`)))

(event `QuickResetPins`
  (`self.ResetPins`))

(event `OnStartNextTurn`
  ;[1 1 1] TODO: Move Control of this to Game Mode
  (`self.ResetPins`))

(event `OnClearPins`
  (`self.RaiseStandingPins`)
  (`KismetSystemLibrary.Delay` 2.0)
  (`self.SweepPins`)
  (`KismetSystemLibrary.Delay` 2.0)
  (`self.LowerStandingPins`)
  (`KismetSystemLibrary.Delay` 2.0)
  (`/Game/BluePrints/BowlingGameMode_BP.ClearPinsComplete` (stale `self.ReceiveBeginPlay` _asbowling_game_mode_bp)))

(event `OnReportPins`
  (`self.ReportPins`))

(event `self.SweepPins`
  (`PrimitiveComponent.SetCollisionEnabled` (`self.Cube`) "QueryAndPhysics")
  (`SceneComponent.SetVisibility` (`self.Cube`) true true)
  (`TweenFunctionLibrary.DueMove` (`self.Cube`) "1.0f" (`KismetMathLibrary.MakeVector` 113.0 0.0 -65.0) "EaseInOut")
  (`TweenFunctionLibrary.DueMove` (`self.Cube`) "1.0f" (`KismetMathLibrary.MakeVector` 0.0 0.0 -65.0) "EaseInOut")
  (`PrimitiveComponent.SetCollisionEnabled` (`self.Cube`) "NoCollision")
  (`SceneComponent.SetVisibility` (`self.Cube`) false true))

(fn `UserConstructionScript`)