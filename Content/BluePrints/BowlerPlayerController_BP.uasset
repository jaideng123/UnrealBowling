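; Player controller for a bowling game that creates and owns the player's UI widgets.
; On BeginPlay it adds the visible bowling HUD, a hidden tutorial widget and a strike display layered above them to the viewport.
; Custom events switch the HUD between pre-bowl, control and end layouts or toggle its visibility, leaving the layout logic to the HUD widget.
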(event `self.ReceiveBeginPlay`
  (bind _returnvalue (`|CreateWidget` "/Game/UI/BowlingHUD.BowlingHUD_C" self))
  (`UserWidget.AddToViewport` _returnvalue 0)
  (`Widget.SetVisibility` _returnvalue "Visible")
  (bind _returnvalue_2 (`|CreateWidget` "/Game/UI/TutorialWidget_BP.TutorialWidget_BP_C" self))
  (`UserWidget.AddToViewport` _returnvalue_2 -1)
  (`Widget.SetVisibility` _returnvalue_2 "Hidden")
  (set `self.TutorialWidget` _returnvalue_2)
  (bind _returnvalue_3 (`|CreateWidget` "/Game/UI/StrikeDisplayUI_BP.StrikeDisplayUI_BP_C" self))
  (`UserWidget.AddToViewport` _returnvalue_3 1))

(event `self.ShowControlUI`
  (`/Game/UI/BowlingHUD.ShowPrimaryUI` (stale `self.ReceiveBeginPlay` _returnvalue)))

(event `self.ShowPreBowlUI`
  (`/Game/UI/BowlingHUD.ShowPreBowlUI` (stale `self.ReceiveBeginPlay` _returnvalue)))

(event `self.ShowEndUI`
  (`/Game/UI/BowlingHUD.ShowEndUI` (stale `self.ReceiveBeginPlay` _returnvalue)))

(event `self.HideUI`
  (`Widget.SetVisibility` (stale `self.ReceiveBeginPlay` _returnvalue) "Hidden"))

(event `self.ShowUI`
  (`Widget.SetVisibility` (stale `self.ReceiveBeginPlay` _returnvalue) "Visible"))

(fn `UserConstructionScript`)