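; ReverseBallCam is a camera actor that keeps its view pointed at the active ball.
; Each tick, while ActiveBall is valid and active, it rotates its CameraComponent to look at the ball's PhysicsComponent location.
; MakeCameraActive switches player 0's view target to this actor with a short ease-in-out blend.
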(event `self.ReceiveTick`
  (params (DeltaSeconds :type "Float (single-precision)"))
  (bind _cameracomponent (`self.CameraComponent`))
  (bind _activeball (`self.ActiveBall`))
  (if (`KismetSystemLibrary.IsValid` _activeball)
    (if (`BallBase.IsActive` _activeball)
      (`SceneComponent.K2_SetWorldRotation` _cameracomponent (`KismetMathLibrary.FindLookAtRotation` (`SceneComponent.K2_GetComponentLocation` _cameracomponent) (`SceneComponent.K2_GetComponentLocation` (`BallBase.PhysicsComponent` (`self.ActiveBall`)))) false false))))

(fn `MakeCameraActive`
  (`PlayerController.SetViewTargetWithBlend` (`GameplayStatics.GetPlayerController` 0) self 0.2 "VTBlend_EaseInOut" 1.0 false))

(fn `UserConstructionScript`)