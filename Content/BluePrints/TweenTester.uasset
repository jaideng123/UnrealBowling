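; TweenTester is a test actor that exercises DUETween move and rotate nodes on a Sphere and a Cube using a selectable easing type.
; From BeginPlay, a looping chain moves the Sphere up and back while rotating the Cube to a flipped orientation and back, spaced by short delays and tick waits.
; Disconnected leftovers hold a debug label for the easing name and a pause/resume test on the move handle.
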(event `self.ReceiveBeginPlay`
  (bind _due_easing_type (`self.Due Easing Type`))
  (bind _due_easing_type_2 (`self.Due Easing Type`))
  (`KismetSystemLibrary.Delay` 0.2 :!label _label)
  (`|ExecutionSequence`
    (:`then_0`
      (bind _outhandle (`DUETweenBlueprintFunctionLibrary.DueMove` (`self.Sphere`) "1.0f" (0.0 0.0 120.0) _due_easing_type_2))
      (`KismetSystemLibrary.DelayUntilNextTick`)
      (`KismetSystemLibrary.DelayUntilNextTick`)
      (`|ExecutionSequence`
        (:`then_0`
          (`DUETweenBlueprintFunctionLibrary.DueMove` (`self.Sphere`) "1.0f" (0.0 0.0 0.0) _due_easing_type)
          (goto _label))
        (:`then_1`
          (`DUETweenBlueprintFunctionLibrary.DueRotate` (`self.Cube`) 0.8 (struct) _due_easing_type))))
    (:`then_1`
      (`DUETweenBlueprintFunctionLibrary.DueRotate` (`self.Cube`) 0.8 (struct :`Pitch` 180.0 :`Yaw` 180.0) _due_easing_type_2))))

(fn `UserConstructionScript`)