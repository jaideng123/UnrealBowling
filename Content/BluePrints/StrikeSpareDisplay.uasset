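; Bowling celebration actor that animates a Strike or Spare display, captured by a SceneCapture2D that sees only this actor.
; At BeginPlay it hides both displays at a hidden anchor and binds to the strike and spare events of BowlingGameMode_BP.
; Each event uses Due tweens to move and rotate its display to the display anchor and later back, while playing a celebration sound.
; Both sequences share a yoyo PointLight sweep.
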(event `self.ReceiveBeginPlay`
  (bind _returnvalue (`SceneComponent.GetRelativeTransform` (`self.TargetHiddenAnchor`)))
  (set `SceneCaptureComponent.ShowOnlyActors` (`|MakeArray` self :!type "Actor Object Reference") (`self.SceneCaptureComponent2D`))
  (`SceneComponent.K2_SetRelativeTransform` (`self.StrikeDisplay`) _returnvalue false false)
  (`SceneComponent.K2_SetRelativeTransform` (`self.SpareDisplay`) _returnvalue false false)
  (bind _asbowling_game_mode_bp (cast `/Game/BluePrints/BowlingGameMode_BP` (`GameplayStatics.GetGameMode`)))
  (add `/Game/BluePrints/BowlingGameMode_BP.RunStrikeSequence` _asbowling_game_mode_bp (delegate `OnRunStrikeSequence`))
  (add `/Game/BluePrints/BowlingGameMode_BP.RunSpareSequence` _asbowling_game_mode_bp (delegate `OnRunSpareSequence`)))

(event `OnRunSpareSequence`
  (`|ExecutionSequence`
    (:`then_0`
      (`DUETweenBlueprintFunctionLibrary.DueMove` (`self.SpareDisplay`) 0.5 (`SceneComponent.RelativeLocation` (`self.TargetDisplayAnchor`)) "Linear")
      (`KismetSystemLibrary.Delay` 2.0)
      (`|ExecutionSequence`
        (:`then_0`
          (`DUETweenBlueprintFunctionLibrary.DueMove` (`self.SpareDisplay`) 0.5 (`SceneComponent.RelativeLocation` (`self.TargetHiddenAnchor`)) "Linear"))
        (:`then_1`
          (`KismetSystemLibrary.Delay` 0.0)
          (`DUETweenBlueprintFunctionLibrary.DueRotate` (`self.SpareDisplay`) 0.5 (`SceneComponent.RelativeRotation` (`self.TargetHiddenAnchor`)) "Linear"))))
    (:`then_1`
      (`KismetSystemLibrary.Delay` 0.2)
      (`DUETweenBlueprintFunctionLibrary.DueRotate` (`self.SpareDisplay`) 0.5 (`SceneComponent.RelativeRotation` (`self.TargetDisplayAnchor`)) "Linear"))
    (:`then_2`
      (`GameplayStatics.PlaySound2D` "/Game/Audio/Cues/SpareCelebration.SpareCelebration" 1.0 1.0 0.0 null null))
    (:`then_3`
      (`DUETweenBlueprintFunctionLibrary.DueMove` (`self.PointLight`) 3.0 (9.347511 500.0 0.0) "InOutQuad" 0 0 true :!label _label))))

(event `OnRunStrikeSequence`
  (`|ExecutionSequence`
    (:`then_0`
      (`DUETweenBlueprintFunctionLibrary.DueMove` (`self.StrikeDisplay`) 0.5 (`SceneComponent.RelativeLocation` (`self.TargetDisplayAnchor`)) "Linear")
      (`KismetSystemLibrary.Delay` 2.0)
      (`|ExecutionSequence`
        (:`then_0`
          (`DUETweenBlueprintFunctionLibrary.DueMove` (`self.StrikeDisplay`) 0.5 (`SceneComponent.RelativeLocation` (`self.TargetHiddenAnchor`)) "Linear"))
        (:`then_1`
          (`KismetSystemLibrary.Delay` 0.0)
          (`DUETweenBlueprintFunctionLibrary.DueRotate` (`self.StrikeDisplay`) 0.5 (`SceneComponent.RelativeRotation` (`self.TargetHiddenAnchor`)) "Linear"))))
    (:`then_1`
      (`KismetSystemLibrary.Delay` 0.2)
      (`DUETweenBlueprintFunctionLibrary.DueRotate` (`self.StrikeDisplay`) 0.5 (`SceneComponent.RelativeRotation` (`self.TargetDisplayAnchor`)) "Linear"))
    (:`then_2`
      (`GameplayStatics.PlaySound2D` "/Game/Audio/Cues/StrikeCelebration.StrikeCelebration" 1.0 1.0 0.0 null null))
    (:`then_3`
      (goto _label))))

(fn `UserConstructionScript`)