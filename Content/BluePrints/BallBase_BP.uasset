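; Base bowling ball Blueprint that handles collision response and feedback for pin hits and lane contact.
; While active, physics hits forward pins to OnPinContact, while other contacts pick rate-limited bounce or looping-check rolling audio by vertical impulse.
; Successful pin hits add particles, camera shake, sound and a brief time-dilation hit-stop.
; Game mode bowl complete and reset events deactivate the ball and fade rolling audio.
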(event `self.ReceiveBeginPlay`
  (bind _asbowling_game_mode_bp (cast `/Game/BluePrints/BowlingGameMode_BP` (`GameplayStatics.GetGameMode`)))
  (add `/Game/BluePrints/BowlingGameMode_BP.BowlComplete` _asbowling_game_mode_bp (delegate `OnBowlComplete`))
  (add `/Game/BluePrints/BowlingGameMode_BP.BowlReset` _asbowling_game_mode_bp (delegate `BowlResetEvent`)))

(event `OnBowlComplete`
  (set `self.IsActive` false :!label _label)
  (`AudioComponent.FadeOut` (`self.Rolling Audio`) 0.1 0.0 "Linear"))

(event `BowlResetEvent`
  (goto _label))

(event `self.PhysicsComponent.OnComponentHit`
  (params (HitComponent :type "PrimitiveComponent Object Reference") (OtherActor :type "Actor Object Reference") (OtherComp :type "PrimitiveComponent Object Reference") (NormalImpulse :type "Vector Structure") (Hit :type "HitResult Structure (by ref)"))
  (bind _rolling_audio (`self.Rolling Audio`))
  (if (`self.IsActive`)
    (bind _aspin (cast `Pin` OtherActor)
      (:`then`
        (`self.OnPinContact` _aspin Hit))
      (:`CastFailed`
        (if (> (.z NormalImpulse) 20000.0)
          (`/Engine/EditorBlueprintResources/StandardMacros.DoOnce` false :!label _label_2
            (:`Completed`
              (`AudioComponent.Play` (`self.Bounce Audio`) 0.0)
              (`KismetSystemLibrary.Delay` 0.5)
              (goto _label_2 :!via `Reset`)))
          (elif (not (`AudioComponent.IsPlaying` _rolling_audio))
            (`AudioComponent.Play` _rolling_audio 0.0)))))))

(event `self.OnSuccessfulPinHit`
  (params (pin :type "Pin Object Reference") (hitResult :type "HitResult Structure"))
  (bind (_bblockinghit _binitialoverlap _time _distance _location _impactpoint _normal) (`GameplayStatics.BreakHitResult` hitResult))
  (`parent.OnSuccessfulPinHit` pin hitResult)
  (`NiagaraFunctionLibrary.SpawnSystemAtLocation` "/Game/Particles/PinHitEffect.PinHitEffect" _location (`KismetMathLibrary.FindLookAtRotation` (`KismetMathLibrary.Vector_Zero`) _normal))
  (`CameraShakeSourceComponent.StartCameraShake` :`self` (`self.CameraShakeSource`) :`InCameraShake` "/Game/PinStrikeCameraShake.PinStrikeCameraShake_C")
  (`AudioComponent.Play` (`self.Pin Hit Audio`) 0.0)
  (`/Engine/EditorBlueprintResources/StandardMacros.DoOnce` false :!label _label_3
    (:`Completed`
      (`GameplayStatics.SetGlobalTimeDilation` 0.1)
      (`KismetSystemLibrary.Delay` 0.012)
      (`GameplayStatics.SetGlobalTimeDilation` 1.0)
      (goto _label_3 :!via `Reset`))))

(fn `HandleImpactAudio`
  (params (A :type "Vector Structure"))
  (bind _returnvalue (`KismetMathLibrary.VSize` A))
  (bind _rolling_audio (`self.Rolling Audio`))
  (if (> _returnvalue 20000.0)
    (`KismetSystemLibrary.PrintString` (`KismetStringLibrary.Conv_DoubleToString` _returnvalue) true true (struct :`G` 0.66 :`B` 1.0 :`A` 1.0) _returnvalue)
    (`/Engine/EditorBlueprintResources/StandardMacros.DoOnce` false
      (:`Completed`
        (`AudioComponent.Play` (`self.Bounce Audio`) 0.0)))
    (elif (not (`AudioComponent.IsPlaying` _rolling_audio))
      (`AudioComponent.Play` _rolling_audio 0.0))))

(fn `UserConstructionScript`)