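; MoverBox is an actor that moves endlessly back and forth between its starting location and a configurable offset.
; On BeginPlay it stores its location and waits a configurable start delay, which can stagger its timing.
; It then loops two chained DueMove tween calls, out and back, over the same duration with quadratic ease-in-out.
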(event `self.ReceiveBeginPlay`
  (set `self.StartingLocation` (`self.K2_GetActorLocation`))
  (`KismetSystemLibrary.Delay` (`self.StartOffset`))
  (`TweenFunctionLibrary.DueMove` null (`self.MoveSpeedSec`) (+ (`self.StartingLocation`) (`self.Offset`)) "EaseInOut" "InOutQuad" :!label _label)
  (`TweenFunctionLibrary.DueMove` null (`self.MoveSpeedSec`) (`self.StartingLocation`) "EaseInOut" "InOutQuad")
  (goto _label))

(fn `UserConstructionScript`)