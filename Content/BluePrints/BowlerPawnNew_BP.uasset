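; Bowler pawn Blueprint that adds camera, audio and haptic feedback to its parent's grip, release, move and zoom events.
; It spawns a ball on BeginPlay and binds to BowlingGameMode_BP events, blending the view back to itself and resetting the ball on next turn, pin clear, bowl reset or forceless release.
; Zooming tweens camera FOV and spring arm rotation while toggling BowlingLocked; movement loops a timer-driven tick sound until it stops.
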(event `BowlResetEvent`
  (`PlayerController.SetViewTargetWithBlend` (`GameplayStatics.GetPlayerController` 0) self 0.5 "VTBlend_EaseInOut" 1.0 true)
  (`self.ResetBall`))

(event `self.ReceiveBeginPlay`
  (`self.SpawnNewBall`)
  (bind _asbowling_game_mode_bp (cast `/Game/BluePrints/BowlingGameMode_BP` (`GameplayStatics.GetGameMode`)))
  (add `/Game/BluePrints/BowlingGameMode_BP.StartNextTurn` _asbowling_game_mode_bp (delegate `OnStartNextTurn`))
  (add `/Game/BluePrints/BowlingGameMode_BP.ClearPinsComplete` _asbowling_game_mode_bp (delegate `ClearPinsComplete_Event`))
  (add `/Game/BluePrints/BowlingGameMode_BP.BowlReset` _asbowling_game_mode_bp (delegate `BowlResetEvent`)))

(event `OnStartNextTurn`
  (`PlayerController.SetViewTargetWithBlend` (`GameplayStatics.GetPlayerController` 0) self 0.5 "VTBlend_EaseInOut" 1.0 false :!label _label)
  (`self.ResetBall`))

(event `ClearPinsComplete_Event`
  (goto _label))

(event `self.OnNoReleaseForce`
  (`KismetSystemLibrary.Delay` 1.0)
  (`PlayerController.SetViewTargetWithBlend` (`GameplayStatics.GetPlayerController` 0) self 0.5 "VTBlend_EaseInOut" 1.0 true)
  (`self.ResetBall`))

(event `self.OnGrip`
  (`parent.OnGrip`)
  (`GameplayStatics.PlaySound2D` "/Game/Audio/Input/GripBall.GripBall" 1.0 1.0 0.0 null null)
  (`PlayerController.PlayDynamicForceFeedback` (`GameplayStatics.GetPlayerController` 0) 0.3 0.1 true true true true))

(event `self.OnRelease`
  (`parent.OnRelease`)
  (`GameplayStatics.PlaySound2D` "/Game/Audio/Input/Throw_Object_2.Throw_Object_2" 1.0 3.0 0.0 null null))

(event `self.ZoomIn`
  (`parent.ZoomIn`)
  (`/Engine/EditorBlueprintResources/StandardMacros.DoOnce` false :!label _label_2
    (:`Completed`
      (set `self.OriginalFOV` (`CameraComponent.FieldOfView` (`self.CameraComp`)))
      (set `self.OriginalRotation` (`SceneComponent.RelativeRotation` (`self.SpringArmComp`)))
      (set `self.BowlingLocked` true)
      (`|ExecutionSequence`
        (:`then_0`
          (`TweenFunctionLibrary.DueFloatField` (`self.CameraComp`) "FieldOfView" 0.5 25.0 "Linear"))
        (:`then_1`
          (`TweenFunctionLibrary.DueRotate` (`self.SpringArmComp`) 0.5 (struct :`Pitch` -5.0) "Linear")
          (goto _label_2 :!via `Reset`))))))

(event `self.ZoomOut`
  (`parent.ZoomOut`)
  (`/Engine/EditorBlueprintResources/StandardMacros.DoOnce` false :!label _label_3
    (:`Completed`
      (set `self.BowlingLocked` false)
      (`|ExecutionSequence`
        (:`then_0`
          (`TweenFunctionLibrary.DueFloatField` (`self.CameraComp`) "FieldOfView" 0.5 (`self.OriginalFOV`) "Linear"))
        (:`then_1`
          (`TweenFunctionLibrary.DueRotate` (`self.SpringArmComp`) 0.5 (`self.OriginalRotation`) "Linear")
          (goto _label_3 :!via `Reset`))))))

(event `self.OnMove`
  (params (moveDist :type "Float (single-precision)"))
  (`parent.OnMove` moveDist)
  (if (!= moveDist 0.0)
    (`/Engine/EditorBlueprintResources/StandardMacros.DoOnce` false :!label _label_4
      (:`Completed`
        (`GameplayStatics.PlaySound2D` "/Game/Audio/Input/Tick_Cue.Tick_Cue" 1.0 1.0 0.0 null null :!label _label_5)
        (bind _returnvalue (`KismetSystemLibrary.K2_SetTimerDelegate` (delegate `OnMoveTick`) 0.15 true))
        (goto _label_6 :!via `Reset`)))
    (else
      (`/Engine/EditorBlueprintResources/StandardMacros.DoOnce` false :!label _label_6
        (:`Completed`
          (`KismetSystemLibrary.K2_ClearAndInvalidateTimerHandle` _returnvalue)
          (goto _label_4 :!via `Reset`))))))

(event `OnMoveTick`
  (goto _label_5))

(fn `UserConstructionScript`)