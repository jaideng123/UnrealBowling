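; Pin actor that can be raised and lowered, switching between scripted tweens and physics simulation.
; RaisePin turns off mesh physics, then starts a DueMove to its original spawn X/Y at HeightOffset as absolute Z, plus an eased DueRotate.
; LowerPin eases it back to the OriginalSpawn location and re-enables physics after a short delay.
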(event `self.RaisePin`
  (params (X :type "Float (double-precision)"))
  (`PrimitiveComponent.SetSimulatePhysics` (`self.StaticMeshBody`) false)
  (`|ExecutionSequence`
    (:`then_0`
      (`TweenFunctionLibrary.DueMove` null "1.0f" (`KismetMathLibrary.MakeVector` (.x (`self.K2_GetActorLocation` (`self.OriginalSpawn`))) (.y (`self.K2_GetActorLocation` (`self.OriginalSpawn`))) (`self.HeightOffset`)) "EaseInOut"))
    (:`then_1`
      (`TweenFunctionLibrary.DueRotate` null 0.5 (struct) "EaseIn"))))

(event `self.LowerPin`
  (`TweenFunctionLibrary.DueMove` null "1.0f" (`self.K2_GetActorLocation` (`self.OriginalSpawn`)) "EaseInOut")
  (`KismetSystemLibrary.Delay` 0.1)
  (`PrimitiveComponent.SetSimulatePhysics` (`self.StaticMeshBody`) true))

(fn `UserConstructionScript`)